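; BP_BarDoor is a locked bar door that the player opens with a key, completing a quest.
; Interact checks that the player pawn overlaps the Box and that BP_FirstPersonCharacter has the key, otherwise printing a debug hint.
; DoorSwivel flags the door open and plays a timeline that rotates the mesh 90 degrees on pitch rather than yaw.
; Each timeline update also sets the character's QuestCompleted flag.
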(event Custom|DoorSwivel
  ;[1 1 1] Door Swivel
  (Variables|Default|SetbDoorOpen true)
  (bind _dooropentrack (Timeline|DoorSwivelTimeLine Play)
    (:Update
      (Transformation|SetRelativeRotation (Variables|Default|GetStaticMesh) (Math|Rotator|MakeRotator 0.0 (Math|Float|Lerp 0.0 9e+01 _dooropentrack) 0.0) false false)
      (bind _asbp_first_person_character (Utilities|Casting|CastToBP_FirstPersonCharacter (Game|Player|GetPlayerPawn 0)))
      (Variables|/Game/FirstPerson/Blueprints/BP_FirstPersonCharacter.BP_FirstPersonCharacter_C|SetbQuestCompleted _asbp_first_person_character true))))

(event EventInteract
  ;[1 1 1] Interact
  (if (Collision|IsOverlappingActor (Variables|Default|GetBox) (Game|Player|GetPlayerPawn 0) :!class /Script/Engine.PrimitiveComponent)
    (Development|PrintString "Door")
    (bind _asbp_first_person_character (Utilities|Casting|CastToBP_FirstPersonCharacter (Game|Player|GetPlayerPawn 0)))
    (if (Variables|/Game/FirstPerson/Blueprints/BP_FirstPersonCharacter.BP_FirstPersonCharacter_C|GetbHasKey _asbp_first_person_character)
      (CallFunction|DoorSwivel)
      (else
        (Development|PrintString "GetKey")))))

(fn ConstructionScript)